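; Enemy AI controller that runs the BT_Enemy behavior tree on BeginPlay and feeds perception results into its blackboard.
; Sight updates write the perceived actor to TargetActor only if it casts to MyPlayer.
; Updates from any other sense write the stimulus location to TargetLocation.
; It never checks whether a stimulus was successfully sensed, so losing sight does not clear TargetActor.
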(event `self.ReceiveBeginPlay`
  (`self.RunBehaviorTree` "/Game/Blueprints/BehaviorTrees/BT_Enemy.BT_Enemy"))

(event `self.AIPerception.OnTargetPerceptionUpdated`
  (params (Actor :type "Actor Object Reference") (Stimulus :type "AIStimulus Structure"))
  (set `self.TargetActor` Actor)
  (bind _returnvalue (`AIPerceptionSystem.GetSenseClassForStimulus` Stimulus))
  (if (== _returnvalue "/Script/AIModule.AISense_Sight")
    (bind _asmy_player (cast `MyPlayer` (`self.TargetActor`)))
    (`BlackboardComponent.SetValueAsObject` (`self.Blackboard`) "TargetActor" _asmy_player)
    (else
      (`BlackboardComponent.SetValueAsVector` (`self.Blackboard`) "TargetLocation" (`.StimulusLocation` (break `AIStimulus` Stimulus))))))

(fn `UserConstructionScript`)