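; Melee enemy Blueprint that chases the player once its PawnSensing component spots a pawn.
; Seeing any pawn sets IsSeeingPlayer, which is never cleared here, and calls FollowPlayer.
; FollowPlayer casts the first player character to MyPlayer and issues an AI MoveTo toward it with a short acceptance radius.
; No attack logic is present, and a B key handler only prints a debug string.
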(event `self.PawnSensing.OnSeePawn`
  (params (Pawn :type "Pawn Object Reference"))
  (set `self.isSeeingPlayer` true)
  (`self.FollowPlayer`))

(event `FollowPlayer`
  (if (`self.isSeeingPlayer`)
    (bind _asmy_player (cast `MyPlayer` (`GameplayStatics.GetPlayerCharacter` 0)))
    (`|AIMoveTo` self (0.0 0.0 0.0) _asmy_player 70.0)))

(event `Key|B`
  (params (Key :type "Key Structure"))
  (:`Pressed`
    (`KismetSystemLibrary.PrintString` "Hello")))

(fn `UserConstructionScript`)