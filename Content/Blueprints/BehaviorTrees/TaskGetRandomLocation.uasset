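; Behavior Tree task that picks a random navigable point around the melee enemy for it to use as a target location.
; It randomizes the enemy's walk speed on each run, then writes a point within Radius to the chosen blackboard key.
; The task's success follows the navmesh query's result.
; If the pawn is not a Melee_Enemy_BP, the cast fails and the task never calls FinishExecute.
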(event `self.ReceiveExecuteAI`
  (params (OwnerController :type "AIController Object Reference") (ControlledPawn :type "Pawn Object Reference"))
  (bind _asmelee_enemy_bp (cast `/Game/Blueprints/Enemy/Melee_Enemy_BP` ControlledPawn))
  (`|ExecutionSequence`
    (:`then_0`
      (set `CharacterMovementComponent.MaxWalkSpeed` (`KismetMathLibrary.RandomFloatInRange` 500.0 700.0) (`Character.CharacterMovement` _asmelee_enemy_bp)))
    (:`then_1`
      (bind (_randomlocation _returnvalue) (`NavigationSystemV1.K2_GetRandomLocationInNavigableRadius` (`Actor.K2_GetActorLocation` _asmelee_enemy_bp) (`self.Radius`) null null))
      (`BTFunctionLibrary.SetBlackboardValueAsVector` (`self.blackBoardKey`) _randomlocation)
      (`self.FinishExecute` _returnvalue))))