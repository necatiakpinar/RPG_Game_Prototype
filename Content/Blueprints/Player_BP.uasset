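; Player character Blueprint for a third-person shooter, handling input for shooting, aiming, reloading, crouch, prone and inventory, plus crosshair and quest log HUD creation.
; Shooting delegates to WeaponHandler, while actions record state in the AttributesBoolean struct.
; Aiming slows walking, animates the boom and camera offset with timelines and MoveComponentTo, and, like shooting, locks yaw to the controller.
; Reload holds its flag for the montage's length.
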(event `self.ReceiveBeginPlay`
  (`self.CreateWidgets_BP`))

(event `Key|Tab`
  (params (Key :type "Key Structure"))
  (:`Pressed`
    (`self.ToggleInventory_BP`)))

(event `Key|LeftControl`
  (params (Key :type "Key Structure"))
  (:`Pressed`
    (`self.Prone_BP`)))

(event `Key|R`
  (params (Key :type "Key Structure"))
  (:`Pressed`
    (`self.ReloadMacro`)))

(event `Key|C`
  (params (Key :type "Key Structure"))
  (:`Pressed`
    (`self.Crouch_BP`)))

(event `Key|LeftMouseButton`
  (params (Key :type "Key Structure"))
  (:`Pressed`
    (`self.StartShoot_BP`))
  (:`Released`
    (`self.StopShoot_BP`)))

(event `Key|RightMouseButton`
  (params (Key :type "Key Structure"))
  (:`Pressed`
    (bind _structout (setmembers `AttributesBoolean` :`StructRef` (`self.AttributesBoolean`) :`isAiming` true))
    (if (not (break `AttributesBoolean` _structout))
      (set `CharacterMovementComponent.MaxWalkSpeed` 200.0 (`self.CharacterMovement`))
      (`|ExecutionSequence`
        (:`then_0`
          (bind (_direction _newtrack_0) (`Timeline|Timeline_0` :!via `PlayFromStart`)
            (:`Update`
              (set `SpringArmComponent.TargetArmLength` _newtrack_0 (`self.CameraBoom`)))))
        (:`then_1`
          (`KismetSystemLibrary.MoveComponentTo` (`self.FollowCamera`) (0.0 -10.0 20.0))
          (set `self.bUseControllerRotationYaw` true)))))
  (:`Released`
    (setmembers `AttributesBoolean` :`StructRef` (`self.AttributesBoolean`) :`isAiming` false)
    (set `CharacterMovementComponent.MaxWalkSpeed` (`.movementSpeed` (break `Attributes` (`self.Attributes`))) (`self.CharacterMovement`))
    (`|ExecutionSequence`
      (:`then_0`
        (bind (_direction_2 _newtrack_0_2) (`Timeline|Timeline_1` :!via `ReverseFromEnd`)
          (:`Update`
            (set `SpringArmComponent.TargetArmLength` _newtrack_0_2 (`self.CameraBoom`)))))
      (:`then_1`
        (`KismetSystemLibrary.MoveComponentTo` (`self.FollowCamera`))
        (set `self.bUseControllerRotationYaw` false)))))

(fn `CreateWidgets_BP`
  (`|ExecutionSequence`
    (:`then_0`
      (bind _returnvalue (`|CreateWidget` "/Game/Blueprints/WBP_CrossHair.WBP_CrossHair_C"))
      (`UserWidget.AddToViewport` _returnvalue 0))
    (:`then_1`
      (bind _returnvalue_2 (`|CreateWidget` "/Game/Blueprints/GUI/WBP_QuestLog.WBP_QuestLog_C"))
      (bind _output_get (set `self.QuestLogHUDRef` _returnvalue_2))
      (`UserWidget.AddToViewport` _output_get 0))))

(fn `Crouch_BP`
  (if (`self.bIsCrouched`)
    (`self.UnCrouch`)
    (else
      (`self.Crouch`))))

(fn `Prone_BP`
  (bind _attributesboolean (`self.AttributesBoolean`))
  (if (`.isProning` (break `AttributesBoolean` _attributesboolean))
    (setmembers `AttributesBoolean` :`StructRef` _attributesboolean :`isProning` false)
    (else
      (setmembers `AttributesBoolean` :`StructRef` _attributesboolean :`isProning` true))))

(fn `StartShoot_BP`
  (`WeaponHandlerComponent.StartShooting` (`self.WeaponHandler`))
  (setmembers `AttributesBoolean` :`StructRef` (`self.AttributesBoolean`) :`isAiming` true)
  (set `self.bUseControllerRotationYaw` true))

(fn `StopShoot_BP`
  (`WeaponHandlerComponent.StopShooting` (`self.WeaponHandler`))
  (setmembers `AttributesBoolean` :`StructRef` (`self.AttributesBoolean`) :`isAiming` false)
  (set `self.bUseControllerRotationYaw` false))

(fn `ToggleInventory_BP`
  (bind _returnvalue (`GameplayStatics.GetPlayerController` 0))
  (bind _returnvalue_2 (`|CreateWidget` "/Game/Blueprints/GUI/WBP_Inventory.WBP_Inventory_C" (`GameplayStatics.GetPlayerController` 0)))
  (`UserWidget.AddToViewport` _returnvalue_2 0)
  (set `PlayerController.bShowMouseCursor` true _returnvalue)
  (`WidgetBlueprintLibrary.SetInputMode_UIOnlyEx` _returnvalue _returnvalue_2))

(fn `UserConstructionScript`)